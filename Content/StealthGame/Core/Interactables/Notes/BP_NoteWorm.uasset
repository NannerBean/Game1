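; BP_NoteWorm is an interactable note that displays the W_NoteWorm widget on screen.
; Its Interaction event uses a FlipFlop to alternate between showing the note while ignoring player look and move input, and removing it while restoring input.
; When the player character enters its Box, an interact prompt appears and is removed after a two-second retriggerable delay.
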(event OnComponentBeginOverlap(Box)
  (params (OverlappedComponent :type Primitive%20Component%20Object%20Reference) (OtherActor :type Actor%20Object%20Reference) (OtherComp :type Primitive%20Component%20Object%20Reference) (OtherBodyIndex :type Integer) (bFromSweep :type Boolean) (SweepResult :type Hit%20Result%20Structure%20%28by%20ref%29))
  (Utilities|Casting|CastToBP_ThirdPersonCharacterCustom OtherActor)
  (bind _returnvalue (UserInterface|CreateWidget "/Game/StealthGame/Core/Interactables/WBP_InteractPrompt.WBP_InteractPrompt_C"))
  (UserInterface|Viewport|AddtoViewport _returnvalue 0)
  (Utilities|FlowControl|RetriggerableDelay 2.0)
  (Widget|RemovefromParent _returnvalue))

(event EventInteraction
  (bind _returnvalue (Game|GetPlayerController 0))
  (Utilities|FlowControl|FlipFlop
    (:A
      (bind _returnvalue_2 (UserInterface|CreateWidget "/Game/StealthGame/Core/Interactables/Notes/W_NoteWorm.W_NoteWorm_C"))
      (UserInterface|Viewport|AddtoViewport _returnvalue_2 0)
      (Input|SetIgnoreLookInput _returnvalue true)
      (Input|SetIgnoreMoveInput _returnvalue true))
    (:B
      (Widget|RemovefromParent _returnvalue_2)
      (Input|SetIgnoreLookInput _returnvalue false)
      (Input|SetIgnoreMoveInput _returnvalue false))))

(fn ConstructionScript)