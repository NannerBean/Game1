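; BP_Safe is an interactable safe that opens when the correct passcode is entered.
; Interacting shows the mouse cursor, blocks player move and look input, and adds a WBP_Keypad widget to the viewport.
; A combo input event compares the received code to Passcode; on a match, a Timeline lerps the Door's relative location to slide it along local X.
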(event Custom|Open%20Door
  (bind _newtrack_0 (Timeline|Timeline Play)
    (:Update
      (Transformation|SetRelativeLocation (Variables|Default|GetDoor) (Math|Vector|Lerp(Vector) "0.933671,27.341570,38.549718" "-49.000000,27.341570,38.549718" _newtrack_0) false false))))

(event EventrInput(combo)
  (params (Combo :type String))
  (if (Utilities|Enum|Equal(Enum) Combo (Variables|Default|GetPasscode))
    (Development|PrintString "Opening!!!")
    (CallFunction|OpenDoor)))

(event EventInteraction
  (bind _returnvalue (Game|GetPlayerController 0))
  (Variables|/Script/Engine.PlayerController|SetbShowMouseCursor _returnvalue true)
  (Input|SetIgnoreMoveInput _returnvalue true)
  (Input|SetIgnoreLookInput _returnvalue true)
  (bind _returnvalue_2 (UserInterface|CreateWidget "/Game/StealthGame/Core/Interactables/WBP_Keypad.WBP_Keypad_C"))
  (UserInterface|Viewport|AddtoViewport _returnvalue_2 0))

(fn ConstructionScript)